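; Handgun weapon Blueprint that supplies the animations and sound for firing and reloading.
; Fire and ReloadStart call global fire and reload events, which play the matching animation on both the first-person and third-person meshes.
; Firing also spawns a gunshot sound at the weapon's location.
; The other weapon event hooks, including alt-fire, melee, equip and ammo, are empty.
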(event Custom|Global_Fire_Event
  (Components|Animation|PlayAnimation (Variables|Default|GetMesh1P) "/Game/Rade/Meshes/Weapons/HandGun/HandGun_Fire_Anim.HandGun_Fire_Anim" false)
  (Audio|SpawnSoundatLocation "/Game/Rade/Sounds/Pistol/remingtongunshot_Cue.remingtongunshot_Cue" (Transformation|GetActorLocation)))

(event Custom|Global_Reload_Event
  (Components|Animation|PlayAnimation (Variables|Default|GetMesh1P) "/Game/Rade/Meshes/Weapons/HandGun/HandGun_Reload_anim.HandGun_Reload_anim" false))

(event EventReloadStart
  (CallFunction|GlobalReloadEvent))

(event EventFire
  (CallFunction|GlobalFireEvent))

(event EventItemDroped
  (params (thePickup :type Item%20Pickup%20Object%20Reference)))

(event EventItemUpdated)

(event EventItemUsed)

(event EventAltAmmoUsed)

(event EventAltFire)

(event EventAltFirePressEnd)

(event EventAltFirePressStart)

(event EventAmmoUsed)

(event EventEquipEnd)

(event EventEquipStart)

(event EventFirePressEnd)

(event EventFirePressStart)

(event EventHitEnemy
  (params (HitData :type Hit%20Result%20Structure)))

(event EventMeleeAttack)

(event EventNoAmmo)

(event EventPreAltFire)

(event EventPreFire)

(event EventPreMeleeAttack)

(event EventReloadEnd)

(event EventUnequipEnd)

(event EventUnequipStart)

(fn ConstructionScript)