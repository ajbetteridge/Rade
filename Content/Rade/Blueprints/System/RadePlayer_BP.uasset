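; Player character Blueprint for Rade that handles sprinting, player name and color, and local menu input.
; Name and color come from the game instance, with the color tinting a shared dynamic material on both meshes.
; Timelines ramp walk speed for sprinting, and authority Tick slows it when movement isn't forward.
; It also toggles the HUD options menu, exits on Escape and saves video settings on EndPlay.
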(event Custom|StopSprint_Event
  (bind _charactermovement (Variables|Character|GetCharacterMovement))
  (Utilities|FlowControl|Sequence
    (:then_0
      (bind _movespeed (Timeline|SprintTimeLine Stop)
        (:Update
          (Variables|/Script/Engine.CharacterMovementComponent|SetMaxWalkSpeed _charactermovement _movespeed))))
    (:then_1
      (bind _time (Timeline|DecreseSpeed PlayFromStart)
        (:Update
          (Variables|/Script/Engine.CharacterMovementComponent|SetMaxWalkSpeed _charactermovement (Math|Float|Lerp (Variables|/Script/Engine.CharacterMovementComponent|GetMaxWalkSpeed _charactermovement) 6e+02 _time)))))))

(event Custom|StartSprint_Event
  (bind _charactermovement (Variables|Character|GetCharacterMovement))
  (if (<= (Variables|/Script/Engine.CharacterMovementComponent|GetMaxWalkSpeed (Variables|Character|GetCharacterMovement)) 601.0)
    (bind _movespeed (Timeline|SprintTimeLine PlayFromStart)
      (:Update
        (Variables|/Script/Engine.CharacterMovementComponent|SetMaxWalkSpeed _charactermovement _movespeed)))
    (else
      (Utilities|FlowControl|Sequence
        (:then_0
          (Timeline|SprintTimeLine Stop))
        (:then_1
          (bind _time (Timeline|DecreseSpeed PlayFromStart)
            (:Update
              (Variables|/Script/Engine.CharacterMovementComponent|SetMaxWalkSpeed _charactermovement (Math|Float|Lerp (Variables|/Script/Engine.CharacterMovementComponent|GetMaxWalkSpeed _charactermovement) 6e+02 _time)))))))))

(event EventTick
  (params (DeltaSeconds :type Float%20%28single-precision%29))
  (bind _charactermovement (Variables|Character|GetCharacterMovement))
  (Networking|SwitchHasAuthority
    (:Authority
      (Utilities|FlowControl|Sequence
        (:then_0
          (if (< (Math|Vector|DotProduct (Math|Vector|Normalize (Variables|/Script/Engine.MovementComponent|GetVelocity (Variables|Character|GetCharacterMovement))) (Transformation|GetActorForwardVector)) 0.9)
            (if (not (<= (Variables|/Script/Engine.CharacterMovementComponent|GetMaxWalkSpeed (Variables|Character|GetCharacterMovement)) 601.0))
              (Utilities|FlowControl|Sequence
                (:then_0
                  (bind _movespeed (Timeline|SprintTimeLine Stop)
                    (:Update
                      (Variables|/Script/Engine.CharacterMovementComponent|SetMaxWalkSpeed _charactermovement _movespeed))))
                (:then_1
                  (bind _time (Timeline|DecreseSpeed PlayFromStart)
                    (:Update
                      (Variables|/Script/Engine.CharacterMovementComponent|SetMaxWalkSpeed _charactermovement (Math|Float|Lerp (Variables|/Script/Engine.CharacterMovementComponent|GetMaxWalkSpeed _charactermovement) 6e+02 _time)))))))))
        (:then_1
          (Variables|Default|SetCurrentWalkSpeed (Math|Vector|VectorLength (Transformation|GetVelocity))))))))

(event EventBeginPlay
  (bind _asrade_game_instance (Utilities|Casting|CastToRadeGameInstance (Game|GetGameInstance) :!label _label)
    (:then
      (Networking|SwitchHasAuthority
        (:Authority
          (if (Pawn|IsLocallyControlled)
            (Class|RadeCharacter|SetCharacterStats (Variables|/Script/Rade.RadeGameInstance|GetPlayerName _asrade_game_instance) (Variables|/Script/Rade.RadeGameInstance|GetPlayerColor _asrade_game_instance) :!label _label_2)))
        (:Remote
          (goto _label_2))))
    (:CastFailed
      (Utilities|FlowControl|Delay 0.5)
      (goto _label))))

(event EventAction)

(event EventResetMoveSpeed
  (bind _charactermovement (Variables|Character|GetCharacterMovement))
  (if (not (<= (Variables|/Script/Engine.CharacterMovementComponent|GetMaxWalkSpeed (Variables|Character|GetCharacterMovement)) 601.0))
    (Utilities|FlowControl|Sequence
      (:then_0
        (bind _movespeed (Timeline|SprintTimeLine Stop)
          (:Update
            (Variables|/Script/Engine.CharacterMovementComponent|SetMaxWalkSpeed _charactermovement _movespeed))))
      (:then_1
        (bind _time (Timeline|DecreseSpeed PlayFromStart)
          (:Update
            (Variables|/Script/Engine.CharacterMovementComponent|SetMaxWalkSpeed _charactermovement (Math|Float|Lerp (Variables|/Script/Engine.CharacterMovementComponent|GetMaxWalkSpeed _charactermovement) 6e+02 _time))))))))

(event EventCharacterStatsUpdated
  (Rendering|Material|SetVectorParameterValue (Variables|Default|GetPlayerMat) "Color" (Variables|Default|GetCharacterColor) :!class /Script/Engine.MaterialInstanceDynamic))

(event EventFAction)

(event EventItemDroped
  (params (ThePickup :type Item%20Pickup%20Object%20Reference)))

(event EventItemUsed
  (params (TheItem :type Item%20Object%20Reference)))

(event EventJump)

(event EventMeleeAction)

(event EventPlayerRevived)

(event EventPlayerDied)

(event EventReload)

(event EventToggleInventory)

(event EventEndPlay
  (params (EndPlayReason :type EEndPlayReason%20Enum :default "Destroyed"))
  (Class|OptionManager|SaveVideoModeandQuality))

(event Input|ActionEvents|InputActionOptions
  (params (Key :type Key%20Structure))
  (:Pressed
    (bind _asplayer_controller (Utilities|Casting|CastToPlayerController (Pawn|GetController)))
    (bind _asrade_hud_bp (Utilities|Casting|CastToRadeHUD_BP (HUD|GetHUD _asplayer_controller)))
    (Utilities|IsValid (Variables|/Game/Rade/Blueprints/HUD/RadeHUD_BP.RadeHUD_BP_C|GetMainWidget _asrade_hud_bp)
      (:Is%20Valid
        (Default|ToggleOptionsEvent (Variables|/Game/Rade/Blueprints/HUD/RadeHUD_BP.RadeHUD_BP_C|GetMainWidget _asrade_hud_bp))
        (bind _isa (Utilities|FlowControl|FlipFlop)
          (:A
            _)
          (:B
            _))
        (Input|SetIgnoreLookInput _asplayer_controller _isa)
        (Variables|/Script/Engine.PlayerController|SetbShowMouseCursor _asplayer_controller _isa)))))

(event Input|KeyboardEvents|Escape
  (params (Key :type Key%20Structure))
  (:Pressed
    (bind _asplayer_controller (Utilities|Casting|CastToPlayerController (Pawn|GetController)))
    (Development|ExecuteConsoleCommand "Exit" _asplayer_controller)))

(event Input|KeyboardEvents|LeftShift
  (params (Key :type Key%20Structure))
  (:Pressed
    (CallFunction|StartSprintEvent))
  (:Released
    (CallFunction|StopSprintEvent)))

(fn ConstructionScript
  (bind _returnvalue (Rendering|Material|CreateDynamicMaterialInstance "/Game/Rade/Materials/BasePlayerMaterial_Mat.BasePlayerMaterial_Mat" :!class /Script/Engine.KismetMaterialLibrary))
  (bind _output_get (Variables|Default|SetPlayerMat _returnvalue))
  (Rendering|Material|SetMaterial (Variables|Character|GetMesh) 0 _output_get))