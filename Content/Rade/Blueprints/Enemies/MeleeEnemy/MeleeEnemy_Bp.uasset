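; Melee enemy character that fights with a sword and explodes on permanent death.
; Shortly after BeginPlay, the authority side equips the sword weapon.
; The attack event sets the body anim instance to the melee weapon archetype and plays its Fire state.
; On death, if it cannot revive, it waits briefly, spawns an explosion at the pelvis socket, then destroys its weapon and itself.
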(event Custom|StartAttack_Event
  (bind _bodyaniminstance (Variables|Default|GetBodyAnimInstance))
  (bind _asbody_anim_bp (Utilities|Casting|CastToBody_Anim_BP _bodyaniminstance))
  (Class|RadeAnimInstance|SetAnimArchetype _bodyaniminstance "Melee_Weapon")
  (Default|PlayAnimStateEvent _asbody_anim_bp "Fire"))

(event EventBeginPlay
  (Utilities|FlowControl|Delay 0.2)
  (Networking|SwitchHasAuthority
    (:Authority
      (bind _asweapon (Utilities|Casting|CastToWeapon (Class|RadeData|ObjectfromBlueprint "/Game/Rade/Blueprints/Weapons/Sword_Weapon_BP.Sword_Weapon_BP_C")))
      (Class|RadeCharacter|EquipWeapon _asweapon))))

(event EventCharacterDeath
  (if (not (Variables|Default|GetbCanRevive))
    (Utilities|FlowControl|Delay 2.0)
    (Effects|SpawnEmitteratLocation "/Game/Rade/Particles/P_Explosion.P_Explosion" (+ (Transformation|GetSocketLocation (Variables|Character|GetMesh) "pelvisSocket") "0, 0,20.000000"))
    (Actor|DestroyActor (Variables|Default|GetTheWeapon))
    (Actor|DestroyActor)))

(fn ConstructionScript)