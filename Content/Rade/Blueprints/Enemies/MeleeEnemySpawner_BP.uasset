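; MeleeEnemySpawner_BP is a server-side spawner that keeps up to a maximum number of melee enemies alive at its location.
; On BeginPlay with authority, one looping timer spawns a MeleeEnemy_BP plus its controller, which possesses it, whenever the tracked list is below the cap.
; A second looping timer prunes invalid entries from the list, freeing slots for replacement spawns.
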(event Custom|SpawnEnemy_Event
  (if (< (Utilities|Array|Length (Variables|Default|GetSpawnedActors)) (Variables|Default|GetMaxEnemyNumber))
    (bind _returnvalue (Game|SpawnActorfromClass "/Game/Rade/Blueprints/Enemies/MeleeEnemy/MeleeEnemy_Bp.MeleeEnemy_BP_C" (Transformation|GetActorTransform) "Undefined" 0 0))
    (Utilities|Array|Add (Variables|Default|GetSpawnedActors) _returnvalue)
    (bind _returnvalue_2 (Game|SpawnActorfromClass "/Game/Rade/Blueprints/Enemies/MeleeEnemy/MeleeEnemy_Controller_BP.MeleeEnemy_Controller_BP_C" (Transformation|GetActorTransform) "Undefined" 0 0))
    (Pawn|Possess _returnvalue_2 _returnvalue)))

(event Custom|CheckEnemyList_Event
  (bind _spawnedactors (Variables|Default|GetSpawnedActors))
  (for (_array_element _array_index) _spawnedactors
    (Utilities|IsValid _array_element
      (:Is%20Not%20Valid
        (Utilities|Array|RemoveIndex _spawnedactors _array_index)))))

(event EventBeginPlay
  (Networking|SwitchHasAuthority
    (:Authority
      (Utilities|Time|SetTimerbyEvent (delegate Custom|SpawnEnemy_Event) (Variables|Default|GetSpawnDelay) true)
      (Utilities|Time|SetTimerbyEvent (delegate Custom|CheckEnemyList_Event) (Variables|Default|GetDeathCheckSpeed) true))))

(fn ConstructionScript)