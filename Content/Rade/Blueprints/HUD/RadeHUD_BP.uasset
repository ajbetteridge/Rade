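; RadeHUD_BP is the HUD Blueprint that creates the main HUD widget and relays inventory and weapon UI events to it.
; On BeginPlay it retries every second until the RadePC_BP controller and player are valid, then creates, initialises and displays the widget with references to itself and the controller.
; Its events forward inventory toggle, update and scroll, plus weapon status updates, to the main widget or its child widgets.
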(event EventBeginPlay
  (bind _asrade_pc_bp (Utilities|Casting|CastToRadePC_BP (Game|Player|GetOwningPlayerController) :!label _label)
    (:then
      (bind _output_get (Variables|Default|SetThePC _asrade_pc_bp))
      (Utilities|IsValid (Class|BaseHUD|GetPlayer) :!label _label_2
        (:Is%20Valid
          (bind _returnvalue (UserInterface|CreateWidget "/Game/Rade/Blueprints/HUD/MainHUDWidget.MainHUDWidget_C" _output_get))
          (Variables|Default|SetMainWidget _returnvalue)
          (Variables|/Game/Rade/Blueprints/HUD/MainHUDWidget.MainHUDWidget_C|SetTheHUD (Variables|Default|GetMainWidget) self)
          (Variables|/Game/Rade/Blueprints/HUD/MainHUDWidget.MainHUDWidget_C|SetThePC (Variables|Default|GetMainWidget) (Variables|Default|GetThePC))
          (Default|InitialiseWidgetEvent (Variables|Default|GetMainWidget))
          (UserInterface|Viewport|AddtoViewport (Variables|Default|GetMainWidget) 0))
        (:Is%20Not%20Valid
          (Utilities|FlowControl|Delay 1.0)
          (goto _label_2))))
    (:CastFailed
      (Utilities|FlowControl|Delay 1.0)
      (goto _label))))

(event EventWeaponUpdated
  (bind _mainwidget (Variables|Default|GetMainWidget))
  (bind _weaponwidget (Variables|/Game/Rade/Blueprints/HUD/MainHUDWidget.MainHUDWidget_C|GetWeaponWidget _mainwidget))
  (Utilities|IsValid _mainwidget
    (:Is%20Valid
      (Utilities|IsValid _weaponwidget
        (:Is%20Valid
          (Default|UpdateStatusEvent _weaponwidget))))))

(event EventInventoryScrollDown
  (bind _mainwidget (Variables|Default|GetMainWidget))
  (bind _inventorywidget (Variables|/Game/Rade/Blueprints/HUD/MainHUDWidget.MainHUDWidget_C|GetInventoryWidget _mainwidget))
  (Utilities|IsValid _inventorywidget
    (:Is%20Valid
      (Default|ScrollDownEvent _inventorywidget))))

(event EventInventoryScrollUp
  (bind _mainwidget (Variables|Default|GetMainWidget))
  (bind _inventorywidget (Variables|/Game/Rade/Blueprints/HUD/MainHUDWidget.MainHUDWidget_C|GetInventoryWidget _mainwidget))
  (Utilities|IsValid _inventorywidget
    (:Is%20Valid
      (Default|ScrollUpEvent _inventorywidget))))

(event EventInventoryToggled
  (bind _mainwidget (Variables|Default|GetMainWidget))
  (Utilities|IsValid _mainwidget
    (:Is%20Valid
      (Default|InventoryToggleEvent _mainwidget))))

(event EventInventoryUpdated
  (bind _mainwidget (Variables|Default|GetMainWidget))
  (Utilities|IsValid _mainwidget
    (:Is%20Valid
      (Default|InventoryUpdatedEvent _mainwidget))))

(fn ConstructionScript)